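; Actor component that opens a level by name after a delay, with an optional loading screen.
; StartTransition sets a timer that fires SwitchLevel and, if requested, adds WBP_LoadingScreen to the viewport.
; A looping timer steps the widget's Alpha up until it reaches full, then pauses itself, running independently of the switch delay.
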(event `SwitchLevel`
  (`GameplayStatics.OpenLevel` (stale `StartTransition` `Level Name`)))

(event `StartTransition`
  (params (`Level Name` :type Name) (Delay :type "Float (double-precision)" :default 1.0) (`Show Loading Screen` :type Boolean :default true))
  (`KismetSystemLibrary.K2_SetTimerDelegate` (delegate `SwitchLevel`) Delay)
  (if `Show Loading Screen`
    (bind _returnvalue (`|CreateWidget` "/Game/Game/UI/Widgets/WBP_LoadingScreen.WBP_LoadingScreen_C" (`GameplayStatics.GetPlayerController` 0)))
    (`UserWidget.AddToViewport` _returnvalue 3)
    (bind _returnvalue_2 (`KismetSystemLibrary.K2_SetTimerDelegate` (delegate `UpdateLoadingScreen`) 0.01 true))))

(event `UpdateLoadingScreen`
  (bind _output_get (set `/Game/Game/UI/Widgets/WBP_LoadingScreen.Alpha` (+ (`/Game/Game/UI/Widgets/WBP_LoadingScreen.Alpha` (stale `StartTransition` _returnvalue)) 0.01) (stale `StartTransition` _returnvalue)))
  (if (>= _output_get 1.0)
    (`KismetSystemLibrary.K2_PauseTimerHandle` (stale `StartTransition` _returnvalue_2))))