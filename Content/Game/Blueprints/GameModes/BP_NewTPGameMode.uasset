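; Third-person game mode that handles player respawn after a ragdoll and can open the Lvl_ThirdPerson level.
; StartRespawn disables input, ragdolls the controlled BP_ThirdPersonCharacter, then after a short delay destroys the pawn and restarts the player.
; It then resets the ACHealth component on BP_PlayerState, always taken from player index 0 rather than the respawning controller.
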(event `LoadLevel`
  (`GameplayStatics.OpenLevelBySoftObjectPtr` "/Game/Game/Maps/Lvl_ThirdPerson.Lvl_ThirdPerson"))

(event `StartRespawn`
  (params (PlayerController :type "PlayerController Object Reference"))
  (bind _output_get (set `self.PlayerController` PlayerController))
  (`self.DisableInput` _output_get _output_get)
  (bind _returnvalue (`Controller.K2_GetPawn` _output_get))
  (bind _asbp_third_person_character (cast `/Game/Game/Blueprints/Pawns_Characters/Player/BP_ThirdPersonCharacter` _returnvalue))
  (`/Game/Game/Blueprints/Pawns_Characters/Player/BP_ThirdPersonCharacter.StartRagdoll` _asbp_third_person_character)
  (`KismetSystemLibrary.Delay` 3.0)
  (`self.K2_DestroyActor` _returnvalue)
  (`self.RestartPlayer` _output_get)
  (bind _asbp_player_state (cast `/Game/Game/Blueprints/PlayerStates/BP_PlayerState` (`GameplayStatics.GetPlayerState` 0)))
  (`/Game/Game/Blueprints/Components/AC_Health.ResetHealth` (`/Game/Game/Blueprints/PlayerStates/BP_PlayerState.AC_Health` _asbp_player_state)))

(fn `UserConstructionScript`)