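; Game mode for the main menu that shows the WBP_MainMenu widget and handles starting a new game.
; On BeginPlay it creates the menu for the first player controller and adds it to the viewport.
; StartGame resets health and the CLMorts and CLTemps counters in BP_GameInstance, then has the ACLevelSwitcher component transition to Lvl_ThirdPerson with a delay and loading screen.
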(event `self.ReceiveBeginPlay`
  (bind _returnvalue (`|CreateWidget` "/Game/Game/UI/Widgets/WBP_MainMenu.WBP_MainMenu_C" (`GameplayStatics.GetPlayerController` 0)))
  (`UserWidget.AddToViewport` _returnvalue 0))

(event `Start Game`
  (bind _asbp_game_instance (cast `/Game/Game/Blueprints/BP_GameInstance` (`GameplayStatics.GetGameInstance`)))
  (set `/Game/Game/Blueprints/BP_GameInstance.HealthInitialized_GI` false _asbp_game_instance)
  (bind _output_get (set `/Game/Game/Blueprints/BP_GameInstance.MaxHealth_GI` 100.0 _asbp_game_instance))
  (set `/Game/Game/Blueprints/BP_GameInstance.CurrentHealth_GI` _output_get _asbp_game_instance)
  (set `/Game/Game/Blueprints/BP_GameInstance.CL_Morts` 0 _asbp_game_instance)
  (set `/Game/Game/Blueprints/BP_GameInstance.CL_Temps` 0.0 _asbp_game_instance)
  (`/Game/Game/Blueprints/Components/AC_LevelSwitcher.StartTransition` (`self.AC_LevelSwitcher`) "Lvl_ThirdPerson" 1.0 true))

(fn `UserConstructionScript`)