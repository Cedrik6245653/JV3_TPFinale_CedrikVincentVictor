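; BP_VG_Wall is a wall actor that moves away and is removed once the game instance's VGCoins count reaches exactly four.
; A looping one-second timer started on BeginPlay polls the count and plays the WallDisappear timeline.
; Each timeline update lerps the mesh from its current transform toward a hard-coded world transform, clears the timer and triggers a short delay before destroying the actor.
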(event `self.ReceiveBeginPlay`
  (bind _returnvalue (`KismetSystemLibrary.K2_SetTimerDelegate` (delegate `CheckCup`) 1.0 true)))

(event `CheckCup`
  (bind _asbp_game_instance (cast `/Game/Game/Blueprints/BP_GameInstance` (`GameplayStatics.GetGameInstance`)))
  (if (== (`/Game/Game/Blueprints/BP_GameInstance.VG_Coins` _asbp_game_instance) 4.0)
    (bind (_direction _alpha) (`Timeline|WallDisappear` :!via `PlayFromStart`)
      (:`Update`
        (`SceneComponent.K2_SetWorldTransform` (`self.09a-lowpoly-250726`) (`KismetMathLibrary.TLerp` (`SceneComponent.K2_GetComponentToWorld` (`self.09a-lowpoly-250726`)) (`KismetMathLibrary.MakeTransform` (1368.384616 -168.099711 332.540063) (struct :`Yaw` 90.0)) _alpha) false false)
        (`KismetSystemLibrary.K2_InvalidateTimerHandle` (stale `self.ReceiveBeginPlay` _returnvalue))
        (`KismetSystemLibrary.Delay` 1.0)
        (`self.K2_DestroyActor`)))))

(fn `UserConstructionScript`)