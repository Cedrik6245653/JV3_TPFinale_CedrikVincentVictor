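; BP_RocheRoulante is a rolling rock hazard that damages the player on contact.
; When the first player's pawn overlaps it, it passes its Damage value to the ACHealth component on BP_PlayerState, then destroys itself.
; A delay started on BeginPlay also destroys the rock after a fixed lifetime.
; The Blueprint's graphs contain no movement logic.
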(event `self.ReceiveActorBeginOverlap`
  (params (OtherActor :type "Actor Object Reference"))
  ; Dégat causé par la roche
  (if (== OtherActor (`GameplayStatics.GetPlayerPawn` 0))
    (bind _asbp_player_state (cast `/Game/Game/Blueprints/PlayerStates/BP_PlayerState` (`GameplayStatics.GetPlayerState` 0)))
    (message `/Game/Game/Blueprints/Interfaces/BPI_Damagable.TakeDamage` (`/Game/Game/Blueprints/PlayerStates/BP_PlayerState.AC_Health` _asbp_player_state) (`self.Damage`))
    (`self.K2_DestroyActor`)))

(event `self.ReceiveBeginPlay`
  ; Code Pour retirer les roches après un certain temps
  (`KismetSystemLibrary.Delay` 10.0)
  (`self.K2_DestroyActor`))

(fn `UserConstructionScript`)