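; BP_VG_Cup is an interactable cup that appears once the player's VGCoins count on the game instance reaches exactly three.
; A looping one-second timer polls the count, then plays the CupAppear timeline and is cleared.
; The timeline lerps the interact UI, trigger and mesh from the Icon's transform to a hardcoded, scaled-up transform.
; Interacting runs the parent logic, increments VGCoins and destroys the actor.
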(event `self.ReceiveBeginPlay`
  (`parent.ReceiveBeginPlay`)
  (bind _returnvalue (`KismetSystemLibrary.K2_SetTimerDelegate` (delegate `CheckCoins`) 1.0 true)))

(event `CheckCoins`
  (bind _asbp_game_instance (cast `/Game/Game/Blueprints/BP_GameInstance` (`GameplayStatics.GetGameInstance`)))
  (if (== (`/Game/Game/Blueprints/BP_GameInstance.VG_Coins` _asbp_game_instance) 3.0)
    (bind (_direction _alpha) (`Timeline|CupAppear` :!via `PlayFromStart`)
      (:`Update`
        (`SceneComponent.K2_SetWorldTransform` (`self.InteractUI`) (`KismetMathLibrary.TLerp` (`SceneComponent.K2_GetComponentToWorld` (`self.Icon`)) (`KismetMathLibrary.MakeTransform` (240.0 -170.0 105.017763) (struct) (3.0 3.0 3.0)) _alpha) false false)
        (`SceneComponent.K2_SetWorldTransform` (`self.InteractTrigger`) (`KismetMathLibrary.TLerp` (`SceneComponent.K2_GetComponentToWorld` (`self.Icon`)) (`KismetMathLibrary.MakeTransform` (240.0 -170.0 105.017763) (struct) (3.0 3.0 3.0)) _alpha) false false)
        (`SceneComponent.K2_SetWorldTransform` (`self.InteractMesh`) (`KismetMathLibrary.TLerp` (`SceneComponent.K2_GetComponentToWorld` (`self.Icon`)) (`KismetMathLibrary.MakeTransform` (240.0 -170.0 105.017763) (struct) (3.0 3.0 3.0)) _alpha) false false)
        (`KismetSystemLibrary.K2_ClearAndInvalidateTimerHandle` (stale `self.ReceiveBeginPlay` _returnvalue))))))

(fn `Interact`
  (params (Character :type "/Game/Game/Blueprints/Pawns_Characters/Player/BP_ThirdPersonCharacter Object Reference"))
  (`parent.Interact` Character)
  (bind _asbp_game_instance (cast `/Game/Game/Blueprints/BP_GameInstance` (`GameplayStatics.GetGameInstance`)))
  (set `/Game/Game/Blueprints/BP_GameInstance.VG_Coins` (+ (`/Game/Game/Blueprints/BP_GameInstance.VG_Coins` _asbp_game_instance) 1.0) _asbp_game_instance)
  (`self.K2_DestroyActor`))

(fn `UserConstructionScript`
  (`parent.UserConstructionScript`))