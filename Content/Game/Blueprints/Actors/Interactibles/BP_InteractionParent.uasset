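; Base interactable actor with a mesh, a sphere trigger and a widget that shows an interaction description.
; The construction script applies exposed mesh, trigger and UI settings, and BeginPlay passes the description text to WBP_InteractionUI.
; Both begin and end overlap call AddInteraction on BP_ThirdPersonCharacter, so leaving never calls a removal.
; ToggleUI sets widget visibility, while Interact only stores the interacting character.
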(event `self.ReceiveBeginPlay`
  (bind _aswbp_interaction_ui (cast `/Game/Game/UI/Widgets/WBP_InteractionUI` (`WidgetComponent.GetUserWidgetObject` (`self.InteractUI`))))
  (`/Game/Game/UI/Widgets/WBP_InteractionUI.Set Interaction Description` _aswbp_interaction_ui (`self.UIDescription`)))

(event `self.InteractTrigger.OnComponentBeginOverlap`
  (params (OverlappedComponent :type "PrimitiveComponent Object Reference") (OtherActor :type "Actor Object Reference") (OtherComp :type "PrimitiveComponent Object Reference") (OtherBodyIndex :type Integer) (bFromSweep :type Boolean) (SweepResult :type "HitResult Structure (by ref)"))
  (bind _asbp_third_person_character (cast `/Game/Game/Blueprints/Pawns_Characters/Player/BP_ThirdPersonCharacter` OtherActor))
  (`/Game/Game/Blueprints/Pawns_Characters/Player/BP_ThirdPersonCharacter.AddInteraction` _asbp_third_person_character self))

(event `self.InteractTrigger.OnComponentEndOverlap`
  (params (OverlappedComponent :type "PrimitiveComponent Object Reference") (OtherActor :type "Actor Object Reference") (OtherComp :type "PrimitiveComponent Object Reference") (OtherBodyIndex :type Integer))
  (bind _asbp_third_person_character (cast `/Game/Game/Blueprints/Pawns_Characters/Player/BP_ThirdPersonCharacter` OtherActor))
  (`/Game/Game/Blueprints/Pawns_Characters/Player/BP_ThirdPersonCharacter.AddInteraction` _asbp_third_person_character self))

(fn `Interact`
  (params (Character :type "/Game/Game/Blueprints/Pawns_Characters/Player/BP_ThirdPersonCharacter Object Reference"))
  (set `self.InteractCharacter` Character))

(fn `SetupMesh`
  (`StaticMeshComponent.SetStaticMesh` (`self.InteractMesh`) (`self.InteractionMesh`))
  (`SceneComponent.K2_SetRelativeTransform` (`self.InteractMesh`) (`self.MeshTransform`) false false))

(fn `SetupTrigger`
  (`SphereComponent.SetSphereRadius` (`self.InteractTrigger`) (`self.TriggerRadius`) true)
  (`SceneComponent.K2_SetRelativeLocation` (`self.InteractTrigger`) (`self.TriggerLocation`) false false))

(fn `SetupUI`
  (`SceneComponent.K2_SetRelativeLocation` (`self.InteractUI`) (`self.UILocation`) false false))

(fn `ToggleUI`
  (params (IsVisible :type Boolean))
  (`SceneComponent.SetVisibility` (`self.InteractUI`) IsVisible false))

(fn `UserConstructionScript`
  (`self.SetupMesh`)
  (`self.SetupTrigger`)
  (`self.SetupUI`))