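; BP_Interaction_PillarButton is an interactible button that raises or lowers a linked pillar.
; Its Interact override calls the parent, then flips the Activated flag to choose the direction.
; It instantly offsets the referenced Pillar's static mesh component up or down by HeightLength in world Z, relative to its current location, with no sweep or interpolation.
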(fn `Interact`
  (params (Character :type "/Game/Game/Blueprints/Pawns_Characters/Player/BP_ThirdPersonCharacter Object Reference"))
  (bind _returnvalue (`KismetMathLibrary.MakeVector` 0.0 0.0 (`self.Height Length`)))
  (bind _staticmeshcomponent (`StaticMeshActor.StaticMeshComponent` (`self.Pillar`)))
  (bind _returnvalue_2 (`SceneComponent.K2_GetComponentLocation` _staticmeshcomponent))
  (`parent.Interact` Character)
  ; Quand le bouton a été interagit, on détermine si le pillier doit monter ou déscendre.
  (bind _output_get (set `self.Activated` (not (`self.Activated`))))
  (if _output_get
    ; Appliquer la position décidé du pillier.
    (`SceneComponent.K2_SetWorldLocation` _staticmeshcomponent (+ _returnvalue_2 _returnvalue) false false)
    (else
      (`SceneComponent.K2_SetWorldLocation` _staticmeshcomponent (- _returnvalue_2 _returnvalue) false false))))

(fn `UserConstructionScript`
  (`parent.UserConstructionScript`))